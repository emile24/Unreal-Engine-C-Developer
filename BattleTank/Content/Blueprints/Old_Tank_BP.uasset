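; Old tank Blueprint that provides player-controlled camera aiming around the tank.
; AimAzimuth axis input yaws the AznimuthGimbal and AimElevation pitches the SpringArm as local rotations, both scaled by CameraYSpeed without delta time.
; BeginPlay calls SetBarrel, whose body is not in this graph, and the construction script is empty.
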(event EventBeginPlay
  (Class|Tank|SetBarrel))

(event Input|AxisEvents|InputAxisAimAzimuth
  (params (AxisValue :type Float%20%28single-precision%29))
  ;[1 1 1] Camera Input Binding
  (Transformation|AddLocalRotation (Variables|Default|GetAznimuth%20Gimbal) (Math|Rotator|MakeRotator 0.0 0.0 (* AxisValue (Variables|Default|GetCameraYSpeed))) false false))

(event Input|AxisEvents|InputAxisAimElevation
  (params (AxisValue :type Float%20%28single-precision%29))
  ;[1 1 1] Camera Input Binding
  (Transformation|AddLocalRotation (Variables|Default|GetSpringArm) (Math|Rotator|MakeRotator 0.0 (* AxisValue (Variables|Default|GetCameraYSpeed)) 0.0) false false))

(fn ConstructionScript)