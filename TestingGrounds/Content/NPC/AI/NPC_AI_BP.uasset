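; AI controller for an NPC guard that runs the GuardBehaviour tree on the PatrolData blackboard.
; AI perception writes any sensed actor lacking the "Enemy" tag to the blackboard's enemy key, clearing it when sensing is lost.
; Every tick it sets the controlled Ue4ASP_Character's Aiming and Shooting flags according to whether a focus actor exists.
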(event OnTargetPerceptionUpdated(AIPerception)
  (params (Actor :type Actor%20Object%20Reference) (Stimulus :type AI%20Stimulus%20Structure))
  (bind _enemykey (Variables|Default|GetEnemyKey))
  (bind _blackboardcomp (Variables|Default|GetBlackboardComp))
  (if (not (Actor|ActorHasTag Actor "Enemy"))
    (if (.bSuccessfullySensed (Utilities|Struct|BreakAIStimulus Stimulus))
      (Development|PrintString "Sensed")
      (AI|Components|Blackboard|SetValueasObject _blackboardcomp _enemykey Actor)
      (else
        (Development|PrintString "Not sensed")
        (AI|Components|Blackboard|ClearValue _blackboardcomp _enemykey)))))

(event EventBeginPlay
  (bind _blackboardcomponent (Class|AIController|UseBlackboard "/Game/NPC/AI/PatrolData.PatrolData"))
  (AI|RunBehaviorTree "/Game/NPC/AI/GuardBehaviour.GuardBehaviour")
  (Variables|Default|SetBlackboardComp _blackboardcomponent))

(event EventTick
  (params (DeltaSeconds :type Float%20%28single-precision%29))
  (bind _returnvalue (Class|AIController|GetFocusActor))
  (bind _returnvalue_2 (Utilities|IsValid _returnvalue))
  (bind _asue_4asp_character (Utilities|Casting|CastToUe4ASP_Character (Pawn|GetControlledPawn)))
  (Variables|/Game/NPC/Behaviour/Ue4ASP_Character.Ue4ASP_Character_C|SetAiming _asue_4asp_character _returnvalue_2)
  (Variables|/Game/NPC/Behaviour/Ue4ASP_Character.Ue4ASP_Character_C|SetShooting _asue_4asp_character _returnvalue_2))

(fn ConstructionScript)